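; Ramune obstacle that damages BP_Cat on contact, then destroys itself.
; Four side boxes handle overlaps, each playing a collision sound and calling the cat's stop, damage-blink and damage functions.
; Front and back hits also shove the cat along its local X in opposite directions, while side hits do not.
; Each box's DoOnce precedes the cast, so any first overlapping actor uses it up.
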(event `self.ReceiveTick`
  (params (DeltaSeconds :type "Float (single-precision)")))

(event `self.BoxFront.OnComponentBeginOverlap`
  (params (OverlappedComponent :type "PrimitiveComponent Object Reference") (OtherActor :type "Actor Object Reference") (OtherComp :type "PrimitiveComponent Object Reference") (OtherBodyIndex :type Integer) (bFromSweep :type Boolean) (SweepResult :type "HitResult Structure (by ref)"))
  (`/Engine/EditorBlueprintResources/StandardMacros.DoOnce` false
    (:`Completed`
      (bind _asbp_cat (cast `/Game/Cat/BP_Cat` OtherActor))
      (`GameplayStatics.PlaySound2D` "/Game/Sound/Syoutotu.Syoutotu")
      (`self.K2_AddActorLocalOffset` _asbp_cat (-150.0 0.0 0.0) false false)
      (`/Game/Cat/BP_Cat.StopCat` _asbp_cat)
      (`/Game/Cat/BP_Cat.DamageChikachika` _asbp_cat)
      (`/Game/Cat/BP_Cat.Damage` _asbp_cat)
      (`/Engine/EditorBlueprintResources/StandardMacros.DoOnce` false
        (:`Completed`
          (`self.K2_DestroyActor`))))))

(event `self.BoxBack.OnComponentBeginOverlap`
  (params (OverlappedComponent :type "PrimitiveComponent Object Reference") (OtherActor :type "Actor Object Reference") (OtherComp :type "PrimitiveComponent Object Reference") (OtherBodyIndex :type Integer) (bFromSweep :type Boolean) (SweepResult :type "HitResult Structure (by ref)"))
  (`/Engine/EditorBlueprintResources/StandardMacros.DoOnce` false
    (:`Completed`
      (bind _asbp_cat (cast `/Game/Cat/BP_Cat` OtherActor))
      (`GameplayStatics.PlaySound2D` "/Game/Sound/Syoutotu.Syoutotu")
      (`self.K2_AddActorLocalOffset` _asbp_cat (150.0 0.0 0.0) false false)
      (`/Game/Cat/BP_Cat.StopCat` _asbp_cat)
      (`/Game/Cat/BP_Cat.DamageChikachika` _asbp_cat)
      (`/Game/Cat/BP_Cat.Damage` _asbp_cat)
      (`/Engine/EditorBlueprintResources/StandardMacros.DoOnce` false
        (:`Completed`
          (`self.K2_DestroyActor`))))))

(event `self.BoxLeft.OnComponentBeginOverlap`
  (params (OverlappedComponent :type "PrimitiveComponent Object Reference") (OtherActor :type "Actor Object Reference") (OtherComp :type "PrimitiveComponent Object Reference") (OtherBodyIndex :type Integer) (bFromSweep :type Boolean) (SweepResult :type "HitResult Structure (by ref)"))
  (`/Engine/EditorBlueprintResources/StandardMacros.DoOnce` false
    (:`Completed`
      (bind _asbp_cat (cast `/Game/Cat/BP_Cat` OtherActor))
      (`GameplayStatics.PlaySound2D` "/Game/Sound/Syoutotu.Syoutotu")
      (`/Game/Cat/BP_Cat.StopCat` _asbp_cat)
      (`/Game/Cat/BP_Cat.DamageChikachika` _asbp_cat)
      (`/Game/Cat/BP_Cat.Damage` _asbp_cat)
      (`/Engine/EditorBlueprintResources/StandardMacros.DoOnce` false
        (:`Completed`
          (`self.K2_DestroyActor`))))))

(event `self.BoxRight.OnComponentBeginOverlap`
  (params (OverlappedComponent :type "PrimitiveComponent Object Reference") (OtherActor :type "Actor Object Reference") (OtherComp :type "PrimitiveComponent Object Reference") (OtherBodyIndex :type Integer) (bFromSweep :type Boolean) (SweepResult :type "HitResult Structure (by ref)"))
  (`/Engine/EditorBlueprintResources/StandardMacros.DoOnce` false
    (:`Completed`
      (bind _asbp_cat (cast `/Game/Cat/BP_Cat` OtherActor))
      (`GameplayStatics.PlaySound2D` "/Game/Sound/Syoutotu.Syoutotu")
      (`/Game/Cat/BP_Cat.StopCat` _asbp_cat)
      (`/Game/Cat/BP_Cat.DamageChikachika` _asbp_cat)
      (`/Game/Cat/BP_Cat.Damage` _asbp_cat)
      (`/Engine/EditorBlueprintResources/StandardMacros.DoOnce` false
        (:`Completed`
          (`self.K2_DestroyActor`))))))

(fn `UserConstructionScript`)